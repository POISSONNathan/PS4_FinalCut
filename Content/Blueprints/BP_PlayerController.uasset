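; First-person player controller that handles object interaction and look input.
; When interaction is allowed, the interact button fires a short debug-drawn line trace from the character's camera and calls InteractWithObj on any BP_Interactable hit, passing controller and character.
; Turn and LookUp axes broadcast through event dispatchers instead of applying rotation directly.
; Bind helpers can clear existing listeners before binding, and ResetBinding uses them on BeginPlay to set default handlers.
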(event EventBeginPlay
  (CallFunction|ResetBinding))

(event Input|ActionEvents|InputActionInteractionButton
  (params (Key :type Key%20Structure :default "None"))
  (:Pressed
    (if (Variables|Default|GetcanInteract?)
      (bind _out_hit_hit_actor (CallFunction|CreateLineTrace))
      (bind _asbp_interactable (Utilities|Casting|CastToBP_Interactable _out_hit_hit_actor))
      (Default|InteractwithObj _asbp_interactable self (CallFunction|GetPlayerCharacteras)))))

(event Input|AxisEvents|InputAxisTurn
  (params (AxisValue :type Float%20%28single-precision%29))
  (Default|CallTurn AxisValue))

(event Input|AxisEvents|InputAxisLookUp
  (params (AxisValue :type Float%20%28single-precision%29))
  (Default|CallLookUp AxisValue))

(fn ConstructionScript)

(fn CreateLineTrace
  (bind _asfirst_person_character (CallFunction|GetPlayerCharacteras))
  (bind _firstpersoncamera (Variables|/Game/Blueprints/FirstPersonCharacter.FirstPersonCharacter_C|GetFirstPersonCamera _asfirst_person_character))
  (bind _returnvalue (Transformation|GetWorldLocation _firstpersoncamera))
  (bind _outhit (Collision|LineTraceByChannel _returnvalue (+ _returnvalue (* (Math|Vector|GetForwardVector _firstpersoncamera) 4e+02)) "TraceTypeQuery1" false 0 "ForDuration"))
  (return (.hitactor _outhit)))

(fn BindEventtoTurn
  (params (Clear :type Boolean) (Event :type Delegate%20%28by%20ref%29))
  (Utilities|FlowControl|Sequence
    (:then_0
      (if Clear
        (EventDispatchers|UnbindallEventsfromTurn)))
    (:then_1
      (EventDispatchers|BindEventtoTurn Event))))

(fn BindEventtoLookUp
  (params (Clear :type Boolean) (Event1 :type Delegate%20%28by%20ref%29))
  (Utilities|FlowControl|Sequence
    (:then_0
      (if Clear
        (EventDispatchers|UnbindallEventsfromLookUp)))
    (:then_1
      (EventDispatchers|BindEventtoLookUp Event1))))

(fn ResetBinding
  (CallFunction|BindEventtoTurn true (EventDispatchers|CreateEvent (CallFunction|GetPlayerCharacteras) :!event PlayerTurn))
  (CallFunction|BindEventtoLookUp true (EventDispatchers|CreateEvent (CallFunction|GetPlayerCharacteras) :!event PlayerLookUp)))