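; BP_ChaiseBascule is a map prop that endlessly rocks its ChaiseBascule component (French for rocking chair).
; BeginPlay starts the Move event and stores the component's initial relative rotation.
; A timeline track blends the relative rotation between that start and a small roll offset, and Move calls itself whenever the timeline finishes to loop the motion.
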(event Custom|Move
  (bind _startrotation (Variables|Default|GetstartRotation))
  (bind (_roll _pitch _yaw) (Math|Rotator|BreakRotator _startrotation))
  (bind _newtrack_0 (Timeline|Timeline_0 PlayFromStart)
    (:Update
      (Transformation|SetRelativeRotation (Variables|Default|GetChaiseBascule) (Math|Rotator|Lerp(Rotator) _startrotation (Math|Rotator|MakeRotator (+ _roll 7.5) _pitch _yaw) _newtrack_0) false false))
    (:Finished
      (CallFunction|Move))))

(event EventBeginPlay
  (CallFunction|Move)
  (Variables|Default|SetstartRotation (Variables|/Script/Engine.SceneComponent|GetRelativeRotation (Variables|Default|GetChaiseBascule))))

(fn ConstructionScript)