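; Map object that flashes a spotlight in Morse code to spell the message "This is a TV show".
; BeginPlay calls ShowCode, a hardcoded chain of SetVisibility toggles and Delays with short and long pulses for dots and dashes.
; Longer gaps separate letters and words, and the event calls itself at the end to repeat the message indefinitely.
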(event Custom|ShowCode
  (Utilities|FlowControl|Delay 1.0)
  ;[1 1 1] This
  ;;[1 1 1] t
  (Rendering|SetVisibility (Variables|Default|GetSpotLight) true false)
  (Utilities|FlowControl|Delay 0.5)
  (Rendering|SetVisibility (Variables|Default|GetSpotLight) false false)
  (Utilities|FlowControl|Delay 0.5)
  ;;[1 1 1] h
  (Rendering|SetVisibility (Variables|Default|GetSpotLight) true false)
  (Utilities|FlowControl|Delay 0.2)
  (Rendering|SetVisibility (Variables|Default|GetSpotLight) false false)
  (Utilities|FlowControl|Delay 0.2)
  (Rendering|SetVisibility (Variables|Default|GetSpotLight) true false)
  (Utilities|FlowControl|Delay 0.2)
  (Rendering|SetVisibility (Variables|Default|GetSpotLight) false false)
  (Utilities|FlowControl|Delay 0.2)
  (Rendering|SetVisibility (Variables|Default|GetSpotLight) true false)
  (Utilities|FlowControl|Delay 0.2)
  (Rendering|SetVisibility (Variables|Default|GetSpotLight) false false)
  (Utilities|FlowControl|Delay 0.2)
  (Rendering|SetVisibility (Variables|Default|GetSpotLight) true false)
  (Utilities|FlowControl|Delay 0.2)
  (Rendering|SetVisibility (Variables|Default|GetSpotLight) false false)
  (Utilities|FlowControl|Delay 0.5)
  ;;[1 1 1] i
  (Rendering|SetVisibility (Variables|Default|GetSpotLight) true false)
  (Utilities|FlowControl|Delay 0.2)
  (Rendering|SetVisibility (Variables|Default|GetSpotLight) false false)
  (Utilities|FlowControl|Delay 0.2)
  (Rendering|SetVisibility (Variables|Default|GetSpotLight) true false)
  (Utilities|FlowControl|Delay 0.2)
  (Rendering|SetVisibility (Variables|Default|GetSpotLight) false false)
  (Utilities|FlowControl|Delay 0.5)
  ;;[1 1 1] s
  (Rendering|SetVisibility (Variables|Default|GetSpotLight) true false)
  (Utilities|FlowControl|Delay 0.2)
  (Rendering|SetVisibility (Variables|Default|GetSpotLight) false false)
  (Utilities|FlowControl|Delay 0.2)
  (Rendering|SetVisibility (Variables|Default|GetSpotLight) true false)
  (Utilities|FlowControl|Delay 0.2)
  (Rendering|SetVisibility (Variables|Default|GetSpotLight) false false)
  (Utilities|FlowControl|Delay 0.2)
  (Rendering|SetVisibility (Variables|Default|GetSpotLight) true false)
  (Utilities|FlowControl|Delay 0.2)
  (Rendering|SetVisibility (Variables|Default|GetSpotLight) false false)
  (Utilities|FlowControl|Delay 1.0)
  ;[1 1 1] Is
  ;;[1 1 1] i
  (Rendering|SetVisibility (Variables|Default|GetSpotLight) true false)
  (Utilities|FlowControl|Delay 0.2)
  (Rendering|SetVisibility (Variables|Default|GetSpotLight) false false)
  (Utilities|FlowControl|Delay 0.2)
  (Rendering|SetVisibility (Variables|Default|GetSpotLight) true false)
  (Utilities|FlowControl|Delay 0.2)
  (Rendering|SetVisibility (Variables|Default|GetSpotLight) false false)
  (Utilities|FlowControl|Delay 0.5)
  ;;[1 1 1] s
  (Rendering|SetVisibility (Variables|Default|GetSpotLight) true false)
  (Utilities|FlowControl|Delay 0.2)
  (Rendering|SetVisibility (Variables|Default|GetSpotLight) false false)
  (Utilities|FlowControl|Delay 0.2)
  (Rendering|SetVisibility (Variables|Default|GetSpotLight) true false)
  (Utilities|FlowControl|Delay 0.2)
  (Rendering|SetVisibility (Variables|Default|GetSpotLight) false false)
  (Utilities|FlowControl|Delay 0.2)
  (Rendering|SetVisibility (Variables|Default|GetSpotLight) true false)
  (Utilities|FlowControl|Delay 0.2)
  (Rendering|SetVisibility (Variables|Default|GetSpotLight) false false)
  (Utilities|FlowControl|Delay 1.0)
  ;[1 1 1] A
  ;;[1 1 1] a
  (Rendering|SetVisibility (Variables|Default|GetSpotLight) true false)
  (Utilities|FlowControl|Delay 0.2)
  (Rendering|SetVisibility (Variables|Default|GetSpotLight) false false)
  (Utilities|FlowControl|Delay 0.2)
  (Rendering|SetVisibility (Variables|Default|GetSpotLight) true false)
  (Utilities|FlowControl|Delay 0.5)
  (Rendering|SetVisibility (Variables|Default|GetSpotLight) false false)
  (Utilities|FlowControl|Delay 1.0)
  ;[1 1 1] Tv
  ;;[1 1 1] t
  (Rendering|SetVisibility (Variables|Default|GetSpotLight) true false)
  (Utilities|FlowControl|Delay 0.5)
  (Rendering|SetVisibility (Variables|Default|GetSpotLight) false false)
  (Utilities|FlowControl|Delay 0.5)
  ;;[1 1 1] v
  (Rendering|SetVisibility (Variables|Default|GetSpotLight) true false)
  (Utilities|FlowControl|Delay 0.2)
  (Rendering|SetVisibility (Variables|Default|GetSpotLight) false false)
  (Utilities|FlowControl|Delay 0.2)
  (Rendering|SetVisibility (Variables|Default|GetSpotLight) true false)
  (Utilities|FlowControl|Delay 0.2)
  (Rendering|SetVisibility (Variables|Default|GetSpotLight) false false)
  (Utilities|FlowControl|Delay 0.2)
  (Rendering|SetVisibility (Variables|Default|GetSpotLight) true false)
  (Utilities|FlowControl|Delay 0.2)
  (Rendering|SetVisibility (Variables|Default|GetSpotLight) false false)
  (Utilities|FlowControl|Delay 0.2)
  (Rendering|SetVisibility (Variables|Default|GetSpotLight) true false)
  (Utilities|FlowControl|Delay 0.5)
  (Rendering|SetVisibility (Variables|Default|GetSpotLight) false false)
  (Utilities|FlowControl|Delay 1.0)
  ;[1 1 1] Show
  ;;[1 1 1] s
  (Rendering|SetVisibility (Variables|Default|GetSpotLight) true false)
  (Utilities|FlowControl|Delay 0.2)
  (Rendering|SetVisibility (Variables|Default|GetSpotLight) false false)
  (Utilities|FlowControl|Delay 0.2)
  (Rendering|SetVisibility (Variables|Default|GetSpotLight) true false)
  (Utilities|FlowControl|Delay 0.2)
  (Rendering|SetVisibility (Variables|Default|GetSpotLight) false false)
  (Utilities|FlowControl|Delay 0.2)
  (Rendering|SetVisibility (Variables|Default|GetSpotLight) true false)
  (Utilities|FlowControl|Delay 0.2)
  (Rendering|SetVisibility (Variables|Default|GetSpotLight) false false)
  (Utilities|FlowControl|Delay 0.5)
  ;;[1 1 1] h
  (Rendering|SetVisibility (Variables|Default|GetSpotLight) true false)
  (Utilities|FlowControl|Delay 0.2)
  (Rendering|SetVisibility (Variables|Default|GetSpotLight) false false)
  (Utilities|FlowControl|Delay 0.2)
  (Rendering|SetVisibility (Variables|Default|GetSpotLight) true false)
  (Utilities|FlowControl|Delay 0.2)
  (Rendering|SetVisibility (Variables|Default|GetSpotLight) false false)
  (Utilities|FlowControl|Delay 0.2)
  (Rendering|SetVisibility (Variables|Default|GetSpotLight) true false)
  (Utilities|FlowControl|Delay 0.2)
  (Rendering|SetVisibility (Variables|Default|GetSpotLight) false false)
  (Utilities|FlowControl|Delay 0.2)
  (Rendering|SetVisibility (Variables|Default|GetSpotLight) true false)
  (Utilities|FlowControl|Delay 0.2)
  (Rendering|SetVisibility (Variables|Default|GetSpotLight) false false)
  (Utilities|FlowControl|Delay 0.5)
  ;;[1 1 1] O
  (Rendering|SetVisibility (Variables|Default|GetSpotLight) true false)
  (Utilities|FlowControl|Delay 0.5)
  (Rendering|SetVisibility (Variables|Default|GetSpotLight) false false)
  (Utilities|FlowControl|Delay 0.2)
  (Rendering|SetVisibility (Variables|Default|GetSpotLight) true false)
  (Utilities|FlowControl|Delay 0.5)
  (Rendering|SetVisibility (Variables|Default|GetSpotLight) false false)
  (Utilities|FlowControl|Delay 0.2)
  (Rendering|SetVisibility (Variables|Default|GetSpotLight) true false)
  (Utilities|FlowControl|Delay 0.5)
  (Rendering|SetVisibility (Variables|Default|GetSpotLight) false false)
  (Utilities|FlowControl|Delay 0.5)
  ;;[1 1 1] w
  (Rendering|SetVisibility (Variables|Default|GetSpotLight) true false)
  (Utilities|FlowControl|Delay 0.2)
  (Rendering|SetVisibility (Variables|Default|GetSpotLight) false false)
  (Utilities|FlowControl|Delay 0.2)
  (Rendering|SetVisibility (Variables|Default|GetSpotLight) true false)
  (Utilities|FlowControl|Delay 0.5)
  (Rendering|SetVisibility (Variables|Default|GetSpotLight) false false)
  (Utilities|FlowControl|Delay 0.2)
  (Rendering|SetVisibility (Variables|Default|GetSpotLight) true false)
  (Utilities|FlowControl|Delay 0.5)
  (Rendering|SetVisibility (Variables|Default|GetSpotLight) false false)
  (CallFunction|ShowCode))

(event EventBeginPlay
  (CallFunction|ShowCode))

(fn ConstructionScript)