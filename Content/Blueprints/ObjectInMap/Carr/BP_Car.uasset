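; Car actor that drives along world X with its own camera, serving as a moving sequence that ends in a level change.
; Tick offsets the camera at a fixed rate and the car by Speed per frame, without delta-time scaling, while spinning two pivots.
; ChangeCam ramps Speed above its starting value through a timeline, then loads FirstPersonExampleMap after a short delay.
; Respawn returns the actor to its BeginPlay location.
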(event Custom|Respawn
  (Transformation|SetActorLocation (Variables|Default|GetrespawnPoint) false false))

(event Custom|ChangeCam
  (bind _startspeed (Variables|Default|GetstartSpeed))
  (if (== (Variables|Default|Getspeed) (Variables|Default|GetstartSpeed))
    (bind _newtrack_0 (Timeline|Timeline_0 Play)
      (:Update
        (Variables|Default|Setspeed (Math|Float|Lerp _startspeed (+ _startspeed 1e+01) _newtrack_0)))
      (:Finished
        (Utilities|FlowControl|Delay 0.2)
        (Game|OpenLevel(byName) "FirstPersonExampleMap")))))

(event EventTick
  (params (DeltaSeconds :type Float%20%28single-precision%29))
  (Transformation|AddWorldOffset (Variables|Default|GetCamera) "20.000000,0.000000, 0" false false)
  (Transformation|AddWorldOffset (Variables|Default|GetCar) (Math|Vector|MakeVector (Variables|Default|Getspeed) 0.0 0.0) false false)
  (Transformation|AddLocalRotation (Variables|Default|GetPivot0) "0, 0,7.000000" false false)
  (Transformation|AddLocalRotation (Variables|Default|GetPivot1) "0, 0,7.000000" false false))

(event EventBeginPlay
  (Variables|Default|SetrespawnPoint (Transformation|GetActorLocation))
  (Variables|Default|SetstartSpeed (Variables|Default|Getspeed)))

(fn ConstructionScript)