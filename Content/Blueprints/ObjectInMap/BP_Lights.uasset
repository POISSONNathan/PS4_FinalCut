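; BP_Lights is a map object whose spotlight flickers on and off at random intervals.
; On BeginPlay it hides the spotlight and starts the LightOnOff event.
; That event waits a random delay, shows the light, waits another random delay, hides it, then calls itself to loop forever.
; Separate min and max range variables set how long the off and on phases last.
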(event Custom|LightOnOff
  (Utilities|FlowControl|Delay (Math|Random|RandomFloatinRange (Variables|Default|GetminRangeLightOff) (Variables|Default|GetmaxRangeLightOff)))
  (Rendering|SetVisibility (Variables|Default|GetSpotLight1) true false)
  (Utilities|FlowControl|Delay (Math|Random|RandomFloatinRange (Variables|Default|GetminRangeLightOn) (Variables|Default|GetmaxRangeLightOn)))
  (Rendering|SetVisibility (Variables|Default|GetSpotLight1) false false)
  (CallFunction|LightonOff))

(event EventBeginPlay
  (Rendering|SetVisibility (Variables|Default|GetSpotLight1) false false)
  (CallFunction|LightonOff))

(fn ConstructionScript)