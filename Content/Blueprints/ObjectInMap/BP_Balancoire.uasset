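; BP_Balancoire is a map prop, a swing set ("balançoire") that animates its Left and Right components on an endless loop.
; BeginPlay caches each component's starting relative rotation, then starts the two motions with a short stagger so they move out of phase.
; Each side has its own timeline that drives a rotation lerp toward a pitch offset and replays itself from the start when finished.
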(event Custom|MoveBalancoireDroite
  (bind _startrotateright (Variables|Default|GetstartRotateRight))
  (bind (_roll _pitch _yaw) (Math|Rotator|BreakRotator _startrotateright))
  (bind _newtrack_0 (Timeline|Timeline_1 PlayFromStart)
    (:Update
      (Transformation|SetRelativeRotation (Variables|Default|GetRight) (Math|Rotator|Lerp(Rotator) _startrotateright (Math|Rotator|MakeRotator _roll (+ _pitch 2e+01) _yaw) _newtrack_0) false false))
    (:Finished
      (CallFunction|MoveBalancoireDroite))))

(event Custom|MoveBalancoireGauche
  (bind _startrotateleft (Variables|Default|GetstartRotateLeft))
  (bind (_roll _pitch _yaw) (Math|Rotator|BreakRotator _startrotateleft))
  (bind _newtrack_0 (Timeline|Timeline_0 PlayFromStart)
    (:Update
      (Transformation|SetRelativeRotation (Variables|Default|GetLeft) (Math|Rotator|Lerp(Rotator) _startrotateleft (Math|Rotator|MakeRotator _roll (+ _pitch 2e+01) _yaw) _newtrack_0) false false))
    (:Finished
      (CallFunction|MoveBalancoireGauche))))

(event EventBeginPlay
  (Variables|Default|SetstartRotateLeft (Variables|/Script/Engine.SceneComponent|GetRelativeRotation (Variables|Default|GetLeft)))
  (Variables|Default|SetstartRotateRight (Variables|/Script/Engine.SceneComponent|GetRelativeRotation (Variables|Default|GetRight)))
  (Utilities|FlowControl|Delay 1.0)
  (CallFunction|MoveBalancoireGauche)
  (Utilities|FlowControl|Delay 0.3)
  (CallFunction|MoveBalancoireDroite))

(fn ConstructionScript)