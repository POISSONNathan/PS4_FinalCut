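; Actor Blueprint that switches its point light on when the player enters the house during an event.
; On BeginPlay it binds to the player controller's enter-house event, caches the PointLight's intensity and sets it to zero.
; When that event fires, it waits briefly and restores the cached intensity.
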(event Custom|WhenEnterInHouse
  (Utilities|FlowControl|Delay 2.0)
  (Rendering|Components|Light|SetIntensity (Variables|Default|GetPointLight) (Variables|Default|Getintensity)))

(event EventBeginPlay
  (bind _pointlight (Variables|Default|GetPointLight))
  (EventDispatchers|BindEventtoEnterinHouse (CallFunction|GetPlayerControlleras) (EventDispatchers|CreateEvent :!event Custom|WhenEnterInHouse))
  (Variables|Default|Setintensity (Variables|/Script/Engine.LightComponentBase|GetIntensity _pointlight))
  (Rendering|Components|Light|SetIntensity _pointlight 0.0))

(fn ConstructionScript)