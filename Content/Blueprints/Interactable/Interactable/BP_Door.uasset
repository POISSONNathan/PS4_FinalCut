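; Interactable door that swings open and closed on interaction, optionally requiring a key for the first use.
; A locked door checks the player controller for a key, then either clears the inventory and stays unlocked or briefly shows a UI hint.
; The LerpDoor timeline plays forward or reverse, rotating the Pivot 90 degrees in negative yaw from its BeginPlay rotation.
; Player interaction is disabled until the swing finishes and IsOpen flips.
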(event EventInteractwithObj
  (params (Controller :type BP%20Player%20Controller%20Object%20Reference) (Character :type First%20Person%20Character%20Object%20Reference))
  (bind _asbp_player_controller (CallFunction|GetPlayerControlleras))
  (bind _myui (Variables|/Game/Blueprints/Player/BP_PlayerController.BP_PlayerController_C|GetmyUI _asbp_player_controller))
  (if (Variables|Default|GetneedKey?)
    (if (Variables|/Game/Blueprints/Player/BP_PlayerController.BP_PlayerController_C|GetgetKey? _asbp_player_controller)
      (Default|ClearInventory _asbp_player_controller)
      (Variables|Default|SetneedKey? false)
      (Variables|/Game/Blueprints/Player/BP_PlayerController.BP_PlayerController_C|SetcanInteract? (CallFunction|GetPlayerControlleras) false :!label _label)
      (if (Variables|Default|GetisOpen)
        (bind _newtrack_0 (Timeline|LerpDoor ReverseFromEnd)
          (:Update
            (Transformation|SetRelativeRotation (Variables|Default|GetPivot) (CallFunction|LerpObject _newtrack_0) false false))
          (:Finished
            (if (Variables|Default|GetisOpen)
              (Variables|Default|SetisOpen false)
              (else
                (Variables|Default|SetisOpen true)))
            (Variables|/Game/Blueprints/Player/BP_PlayerController.BP_PlayerController_C|SetcanInteract? (CallFunction|GetPlayerControlleras) true)))
        (else
          (Timeline|LerpDoor PlayFromStart)))
      (else
        (Default|SetInformationText _myui "U need a key to open this door")
        (Utilities|FlowControl|RetriggerableDelay 2.0)
        (Default|SetInformationText _myui)))
    (else
      (goto _label))))

(event EventBeginPlay
  (Variables|Default|SetstartRotation (Variables|/Script/Engine.SceneComponent|GetRelativeRotation (Variables|Default|GetPivot))))

(fn ConstructionScript
  (|CallParentFunction))

(fn LerpObject
  (params (Alpha :type Float%20%28single-precision%29))
  (bind _startrotation (Variables|Default|GetstartRotation))
  (bind (_roll _pitch _yaw) (Math|Rotator|BreakRotator _startrotation))
  (return (Math|Rotator|Lerp(Rotator) _startrotation (Math|Rotator|MakeRotator _roll _pitch (- _yaw 9e+01)) Alpha)))