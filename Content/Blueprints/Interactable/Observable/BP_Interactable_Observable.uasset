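; Interactable observable object that floats up in front of the first-person camera for inspection, then returns to its starting transform.
; Interacting disables the character and plays a timeline that blends from the saved transform to a camera-facing pose, then enables input.
; While open, holding left mouse lets the bound turn event set flags that Tick uses to roll the object.
; The interaction button restores control and reverses a second timeline back.
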(event Custom|TurnFunction
  (params (Val :type Float%20%28single-precision%29))
  ;[1 1 1] Move around object
  (if (Variables|Default|GetleftMouseClick)
    (Variables|Default|SetisRotateRight (> Val 0.0))
    (Variables|Default|SetisRotateLeft (< Val 0.0))))

(event Custom|ResetRotate
  ;[1 1 1] Move around object
  (Variables|Default|SetisRotateRight false)
  (Variables|Default|SetisRotateLeft false))

(event EventBeginPlay
  ;[1 1 1] Start transform
  (Variables|Default|SetstartTransform (Transformation|GetActorTransform)))

(event EventInteractwithObj
  (params (Controller :type BP%20Player%20Controller%20Object%20Reference) (Character :type First%20Person%20Character%20Object%20Reference))
  ;[1 1 1] Start interaction
  (if (not (Variables|Default|GetisOpen))
    (Default|BindEventtoTurn (CallFunction|GetPlayerControlleras) true (EventDispatchers|CreateEvent :!event Custom|TurnFunction))
    (Default|DisableCharandInteract (CallFunction|GetPlayerCharacteras) true)
    (bind _newtrack_0 (Timeline|Lerp PlayFromStart)
      (:Update
        (CallFunction|LerpObject _newtrack_0))
      (:Finished
        (Input|EnableInput (CallFunction|GetPlayerControlleras))
        (Variables|Default|SetisOpen true)))))

(event EventTick
  (params (DeltaSeconds :type Float%20%28single-precision%29))
  (bind _returnvalue (Transformation|GetActorRotation))
  (bind _returnvalue_2 (Transformation|GetActorRotation))
  (bind (_roll _pitch _yaw) (Math|Rotator|BreakRotator _returnvalue))
  (bind (_roll_2 _pitch_2 _yaw_2) (Math|Rotator|BreakRotator _returnvalue_2))
  ;[1 1 1] Move around object
  (Utilities|FlowControl|Sequence
    (:then_0
      (if (Variables|Default|GetisRotateLeft)
        (Transformation|SetActorRelativeRotation (Math|Rotator|MakeRotator (+ _roll -2.0) _pitch _yaw))))
    (:then_1
      (if (Variables|Default|GetisRotateRight)
        (Transformation|SetActorRelativeRotation (Math|Rotator|MakeRotator (+ _roll_2 2.0) _pitch_2 _yaw_2))))))

(event Input|ActionEvents|InputActionInteractionButton
  (params (Key :type Key%20Structure :default "None"))
  ;[1 1 1] End interaction
  (:Pressed
    (if (Variables|Default|GetisOpen)
      (Default|DisableCharandInteract (CallFunction|GetPlayerCharacteras) false)
      (Input|DisableInput (CallFunction|GetPlayerControlleras))
      (Default|ResetBinding (CallFunction|GetPlayerControlleras))
      (bind _newtrack_0 (Timeline|LerpReturnObj ReverseFromEnd)
        (:Update
          (CallFunction|LerpObject _newtrack_0))
        (:Finished
          (Variables|Default|SetisOpen false)
          (CallFunction|ResetRotate))))))

(event Input|MouseEvents|LeftMouseButton
  (params (Key :type Key%20Structure :default "None"))
  ;[1 1 1] Move around object
  (:Pressed
    (Variables|Default|SetleftMouseClick true))
  (:Released
    (Variables|Default|SetleftMouseClick false)
    (CallFunction|ResetRotate)))

(fn ConstructionScript
  (|CallParentFunction))

(fn LerpObject
  (params (LerpValue :type Float%20%28single-precision%29))
  (bind _returnvalue (Transformation|GetActorLocation))
  (bind _asfirst_person_character (CallFunction|GetPlayerCharacteras))
  (bind _firstpersoncamera (Variables|/Game/Blueprints/FirstPersonCharacter.FirstPersonCharacter_C|GetFirstPersonCamera _asfirst_person_character))
  (bind _returnvalue_2 (Transformation|GetWorldLocation _firstpersoncamera))
  (bind _returnvalue_3 (Math|Rotator|FindLookatRotation _returnvalue _returnvalue_2))
  (bind (_roll _pitch _yaw) (Math|Rotator|BreakRotator _returnvalue_3))
  (Transformation|SetActorTransform (Math|Transform|Lerp(Transform) (Variables|Default|GetstartTransform) (Math|Transform|MakeTransform (+ (* (Math|Vector|GetForwardVector _firstpersoncamera) 1e+02) _returnvalue_2) (Math|Rotator|MakeRotator (+ _roll 1.8e+02) (+ _pitch 8e+01) _yaw) (Transformation|GetActorScale3D)) LerpValue)))