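; Interactable object the player can pick up to inspect, with a name, readable text and tutorial UI.
; InteractwithObj disables character input and uses a timeline to lerp the actor in front of the first-person camera, facing it.
; While open, holding left mouse suspends look-up and turn input sets flags that Tick uses to roll the object.
; The interaction button restores control, then either destroys the actor or lerps it back, per KillAfterCheck.
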(event Custom|TurnFunction
  (params (Val :type Float%20%28single-precision%29))
  ;[1 1 1] Move around object
  (if (Variables|Default|GetleftMouseClick)
    (Variables|Default|SetisRotateRight (> Val 0.0))
    (Variables|Default|SetisRotateLeft (< Val 0.0))))

(event Custom|ResetRotate
  ;[1 1 1] Move around object
  (Variables|Default|SetisRotateRight false)
  (Variables|Default|SetisRotateLeft false))

(event EventInteractwithObj
  (params (Controller :type BP%20Player%20Controller%20Object%20Reference) (Character :type First%20Person%20Character%20Object%20Reference))
  (bind _asbp_player_controller (CallFunction|GetPlayerControlleras))
  (bind _uiobservableobject (Variables|/Game/Blueprints/Player/BP_PlayerController.BP_PlayerController_C|GetuiObservableObject _asbp_player_controller))
  ;[1 1 1] Start interaction
  (if (not (Variables|Default|GetisOpen))
    (EventDispatchers|UnbindallEventsfromLookUp Controller)
    (EventDispatchers|UnbindallEventsfromMoveForward Controller)
    (Variables|Default|SetstartTransform (Transformation|GetActorTransform))
    (UserInterface|Viewport|AddtoViewport (Variables|/Game/Blueprints/Player/BP_PlayerController.BP_PlayerController_C|GetuiObservableObject (CallFunction|GetPlayerControlleras)) 0)
    (Default|ChangeImageNameObject _uiobservableobject (Variables|Default|GetimageNameObject))
    (Default|ChangeTexttoRead _uiobservableobject (Variables|Default|GetimageTextToRead))
    (Default|ChangeTutoObject _uiobservableobject (Variables|Default|GetimageTutoObject))
    (Default|BindEventtoTurn (CallFunction|GetPlayerControlleras) true (EventDispatchers|CreateEvent :!event Custom|TurnFunction))
    (Input|DisableInput (CallFunction|GetPlayerCharacteras) 0)
    (bind _newtrack_0 (Timeline|Timeline_0 PlayFromStart)
      (:Update
        (CallFunction|LerpObject _newtrack_0))
      (:Finished
        (Input|EnableInput (CallFunction|GetPlayerControlleras))
        (Variables|Default|SetisOpen true)
        (Default|BindEventtoLookUp (CallFunction|GetPlayerControlleras) false (EventDispatchers|CreateEvent (CallFunction|GetPlayerCharacteras) :!event PlayerLookUp))
        (Variables|Default|SetstartRotation (Transformation|GetActorRotation))))))

(event EventTick
  (params (DeltaSeconds :type Float%20%28single-precision%29))
  (bind _returnvalue (Transformation|GetActorRotation))
  (bind _returnvalue_2 (Transformation|GetActorRotation))
  (bind (_roll _pitch _yaw) (Math|Rotator|BreakRotator _returnvalue))
  (bind (_roll_2 _pitch_2 _yaw_2) (Math|Rotator|BreakRotator _returnvalue_2))
  ;[1 1 1] Move around object
  (Utilities|FlowControl|Sequence
    (:then_0
      (if (Variables|Default|GetisRotateLeft)
        (Transformation|SetActorRelativeRotation (Math|Rotator|MakeRotator (+ _roll -2.0) _pitch _yaw))))
    (:then_1
      (if (Variables|Default|GetisRotateRight)
        (Transformation|SetActorRelativeRotation (Math|Rotator|MakeRotator (+ _roll_2 2.0) _pitch_2 _yaw_2))))))

(event Input|ActionEvents|InputActionInteractionButton
  (params (Key :type Key%20Structure :default "None"))
  ;[1 1 1] End interaction
  (:Pressed
    (Widget|RemovefromParent (Variables|/Game/Blueprints/Player/BP_PlayerController.BP_PlayerController_C|GetuiObservableObject (CallFunction|GetPlayerControlleras)))
    (Input|EnableInput (CallFunction|GetPlayerCharacteras) 0)
    (Input|DisableInput (CallFunction|GetPlayerControlleras))
    (Default|ResetBinding (CallFunction|GetPlayerControlleras))
    (if (Variables|Default|GetkillAfterCheck)
      (Actor|DestroyActor)
      (Variables|/Game/Blueprints/Player/BP_PlayerController.BP_PlayerController_C|SetcanInteract? (CallFunction|GetPlayerControlleras) true :!label _label)
      (else
        (bind _newtrack_0 (Timeline|LerpReturn ReverseFromEnd)
          (:Update
            (CallFunction|LerpObject _newtrack_0))
          (:Finished
            (Variables|Default|SetisOpen false)
            (CallFunction|ResetRotate)
            (goto _label)))))))

(event Input|MouseEvents|LeftMouseButton
  (params (Key :type Key%20Structure :default "None"))
  (bind _asbp_player_controller (CallFunction|GetPlayerControlleras))
  ;[1 1 1] Move around object
  (:Pressed
    (Variables|Default|SetleftMouseClick true)
    (EventDispatchers|UnbindallEventsfromLookUp _asbp_player_controller))
  (:Released
    (Variables|Default|SetleftMouseClick false)
    (CallFunction|ResetRotate)
    (EventDispatchers|BindEventtoLookUp _asbp_player_controller (EventDispatchers|CreateEvent (CallFunction|GetPlayerCharacteras) :!event PlayerLookUp))))

(fn ConstructionScript
  (|CallParentFunction))

(fn LerpObject
  (params (LerpValue :type Float%20%28single-precision%29))
  (bind _returnvalue (Transformation|GetActorLocation))
  (bind _asfirst_person_character (CallFunction|GetPlayerCharacteras))
  (bind _firstpersoncamera (Variables|/Game/Blueprints/Player/FirstPersonCharacter.FirstPersonCharacter_C|GetFirstPersonCamera _asfirst_person_character))
  (bind _returnvalue_2 (Transformation|GetWorldLocation _firstpersoncamera))
  (bind _returnvalue_3 (Math|Rotator|FindLookatRotation _returnvalue _returnvalue_2))
  (bind (_roll _pitch _yaw) (Math|Rotator|BreakRotator _returnvalue_3))
  (Transformation|SetActorTransform (Math|Transform|Lerp(Transform) (Variables|Default|GetstartTransform) (Math|Transform|MakeTransform (+ (* (Math|Vector|GetForwardVector _firstpersoncamera) (Variables|Default|GetdistanceToCamera)) _returnvalue_2) (Math|Rotator|MakeRotator (+ _roll 1.8e+02) (+ _pitch 8e+01) _yaw) (Transformation|GetActorScale3D)) LerpValue)))