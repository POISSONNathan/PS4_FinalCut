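; Observable object Blueprint holding an item the player can take while inspecting it.
; While open, Tick compares the actor's roll to its start rotation and allows taking only beyond the configured angle offsets, toggling the pickup tutorial sprite in the observation UI.
; Pressing TakeObject then calls an empty effect function, presumably a hook for child Blueprints, and destroys the item component.
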(event EventTick
  (params (DeltaSeconds :type Float%20%28single-precision%29))
  (|CallParentFunction DeltaSeconds)
  (if (Variables|Default|GetisOpen)
    (if (or (> (.Roll (Math|Rotator|BreakRotator (Transformation|GetActorRotation))) (+ (.Roll (Math|Rotator|BreakRotator (Variables|Default|GetstartRotation))) (Variables|Default|GetminAngle))) (< (.Roll (Math|Rotator|BreakRotator (Transformation|GetActorRotation))) (- (.Roll (Math|Rotator|BreakRotator (Variables|Default|GetstartRotation))) (Variables|Default|GetmaxAngle))))
      (Variables|Default|SetcanTake true)
      (Default|ChangeTutoPickObj (Variables|/Game/Blueprints/Player/BP_PlayerController.BP_PlayerController_C|GetuiObservableObject (CallFunction|GetPlayerControlleras)) "/Game/Sprite/ObjectTuto/Pick_Sprite.Pick_Sprite")
      (else
        (Variables|Default|SetcanTake false)
        (Default|ChangeTutoPickObj (Variables|/Game/Blueprints/Player/BP_PlayerController.BP_PlayerController_C|GetuiObservableObject (CallFunction|GetPlayerControlleras)))))))

(event Input|ActionEvents|InputActionTakeObject
  (params (Key :type Key%20Structure))
  (:Pressed
    (if (and (Variables|Default|GetisOpen) (Variables|Default|GetcanTake))
      (CallFunction|AddEffectTakeObject)
      (Components|DestroyComponent (Variables|Default|GetonjectToTake)))))

(fn ConstructionScript
  (|CallParentFunction))

(fn AddEffectTakeObject)