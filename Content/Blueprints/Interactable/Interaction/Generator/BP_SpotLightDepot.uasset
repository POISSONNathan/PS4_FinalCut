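; BP_SpotLightDepot is a depot light that serves as either a spotlight or a door diode, selected by the DiodeDoor flag.
; The construction script shows the matching light component, and BeginPlay hides the spotlight and binds to the player controller's depot light event.
; LightOn turns the diode green and nudges it along X, or waits TimeLightOn before showing the spotlight and playing its sound cue.
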(event Custom|LightOn
  (bind _pointlight (Variables|Default|GetPointLight))
  (if (Variables|Default|GetdiodeDoor)
    (Rendering|Components|Light|SetLightColor _pointlight "(R=0.126998,G=1.000000,B=0.000000,A=1.000000)" true)
    (Transformation|AddLocalOffset _pointlight "7.000000, 0, 0" false false)
    (else
      (Utilities|FlowControl|Delay (Variables|Default|GettimeLightOn))
      (Rendering|SetVisibility (Variables|Default|GetSpotLight) true false)
      (Audio|Components|Audio|Play (Variables|Default|GetspotLight_Cue) 0.0))))

(event EventBeginPlay
  (Rendering|SetVisibility (Variables|Default|GetSpotLight) false false)
  (EventDispatchers|BindEventtoLightonDepot (CallFunction|GetPlayerControlleras) (EventDispatchers|CreateEvent :!event Custom|LightOn)))

(fn ConstructionScript
  (if (Variables|Default|GetdiodeDoor)
    (Rendering|SetVisibility (Variables|Default|GetPointLight) true false)
    (Rendering|SetVisibility (Variables|Default|GetSpotLight) false false)
    (else
      (Rendering|SetVisibility (Variables|Default|GetPointLight) false false)
      (Rendering|SetVisibility (Variables|Default|GetSpotLight) true false))))