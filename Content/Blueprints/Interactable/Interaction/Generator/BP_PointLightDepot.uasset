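; BP_PointLightDepot is a depot light that stays dark until a light-on event switches it on.
; On BeginPlay it hides its point light and binds an event to the player controller's depot light-on notification.
; LightOn waits a configurable delay, then shows the light and plays the SpotLightCue sound.
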(event Custom|LightOn
  (Utilities|FlowControl|Delay (Variables|Default|GettimeLightOn))
  (Rendering|SetVisibility (Variables|Default|GetPointLight) true false)
  (Audio|Components|Audio|Play (Variables|Default|GetspotLight_Cue) 0.0))

(event EventBeginPlay
  (Rendering|SetVisibility (Variables|Default|GetPointLight) false false)
  (EventDispatchers|BindEventtoLightonDepot (CallFunction|GetPlayerControlleras) (EventDispatchers|CreateEvent :!event Custom|LightOn)))

(fn ConstructionScript)