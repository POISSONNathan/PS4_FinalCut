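; BP_LightDepot is a depot light that reacts to an event bound through the player controller, serving as either a spotlight or a door diode.
; The construction script uses the DiodeDoor flag to show either the point light or the spotlight, and BeginPlay then hides the spotlight.
; LightOn turns the diode's point light green, or reveals the spotlight after a configurable TimeLightOn delay.
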(event Custom|LightOn
  (if (Variables|Default|GetdiodeDoor)
    (Rendering|Components|Light|SetLightColor (Variables|Default|GetPointLight) "(R=0.126998,G=1.000000,B=0.000000,A=1.000000)" true)
    (else
      (Utilities|FlowControl|Delay (Variables|Default|GettimeLightOn))
      (Rendering|SetVisibility (Variables|Default|GetSpotLight) true false))))

(event EventBeginPlay
  (Rendering|SetVisibility (Variables|Default|GetSpotLight) false false)
  (EventDispatchers|BindEventtoLightonDepot (CallFunction|GetPlayerControlleras) (EventDispatchers|CreateEvent :!event Custom|LightOn)))

(fn ConstructionScript
  (if (Variables|Default|GetdiodeDoor)
    (Rendering|SetVisibility (Variables|Default|GetPointLight) true false)
    (Rendering|SetVisibility (Variables|Default|GetSpotLight) false false)
    (else
      (Rendering|SetVisibility (Variables|Default|GetPointLight) false false)
      (Rendering|SetVisibility (Variables|Default|GetSpotLight) true false))))