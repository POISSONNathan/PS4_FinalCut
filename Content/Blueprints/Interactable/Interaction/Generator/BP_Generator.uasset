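; BP_Generator is a one-shot interactable that tips over by 90 degrees in pitch, then unlocks progress for the interacting controller.
; It caches its starting rotation on BeginPlay, and the first InteractwithObj call sets IsOpen and plays a timeline that lerps the actor's rotation.
; When the timeline finishes, it sets GetKey and CanInteract on the controller and calls CallLightOnDepot.
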(event EventBeginPlay
  (Variables|Default|SetstartRotation (Transformation|GetActorRotation)))

(event EventInteractwithObj
  (params (Controller :type BP%20Player%20Controller%20Object%20Reference) (Character :type First%20Person%20Character%20Object%20Reference))
  (bind _startrotation (Variables|Default|GetstartRotation))
  (bind (_roll _pitch _yaw) (Math|Rotator|BreakRotator _startrotation))
  (if (not (Variables|Default|GetisOpen))
    (Variables|Default|SetisOpen true)
    (bind _newtrack_0 (Timeline|Timeline_0 Play)
      (:Update
        (Transformation|SetActorRotation (Math|Rotator|Lerp(Rotator) _startrotation (Math|Rotator|MakeRotator _roll (+ _pitch -9e+01) _yaw) _newtrack_0)))
      (:Finished
        (Variables|/Game/Blueprints/Player/BP_PlayerController.BP_PlayerController_C|SetgetKey? Controller true)
        (Variables|/Game/Blueprints/Player/BP_PlayerController.BP_PlayerController_C|SetcanInteract? Controller true)
        (Default|CallLightonDepot Controller)))))

(fn ConstructionScript
  (|CallParentFunction))