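; Interactable hinged door that opens and closes on player interaction, optionally requiring a key, which clears the player's inventory when used.
; Timelines lerp door yaw and handle roll from their starting rotations, with swing direction set by InverseRotation, alongside sounds and a locked-handle animation.
; CloseDoorFast shuts the door quickly and blocks further opening.
; AddEffectInteract is an empty hook called on unblocked interactions.
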(event Custom|CloseDoorFast
  (Audio|PlaySound2D (Variables|Default|GetcurrentSoundDoorCloseFast) 1.0 1.0 0.0 0 0)
  (Variables|Default|SetcantOpen true)
  (bind _newtrack_0 (Timeline|Timeline_0 ReverseFromEnd)
    (:Update
      (Transformation|SetRelativeRotation (Variables|Default|GetPivotPorte) (CallFunction|LerpDoor _newtrack_0) false false))))

(event EventInteractwithObj
  (params (Controller :type BP%20Player%20Controller%20Object%20Reference) (Character :type First%20Person%20Character%20Object%20Reference))
  (bind _asbp_player_controller (CallFunction|GetPlayerControlleras))
  (if (Variables|Default|GetcantOpen)
    (Variables|/Game/Blueprints/Player/BP_PlayerController.BP_PlayerController_C|SetcanInteract? (CallFunction|GetPlayerControlleras) true)
    (Audio|PlaySound2D (Variables|Default|GetcurrentSoundDoorLock) 1.0 1.0 0.0 0 0)
    (else
      (CallFunction|AddEffectInteract)
      (if (Variables|Default|GetneedKey?)
        (if (Variables|/Game/Blueprints/Player/BP_PlayerController.BP_PlayerController_C|GetgetKey? _asbp_player_controller)
          (Default|ClearInventory _asbp_player_controller)
          (Variables|Default|SetneedKey? false)
          (if (Variables|Default|GetisOpen) :!label _label
            (Audio|PlaySound2D (Variables|Default|GetcurrentSoundDoorClose) 1.0 1.0 0.0 0 0)
            (bind _newtrack_0 (Timeline|Door ReverseFromEnd)
              (:Update
                (Transformation|SetRelativeRotation (Variables|Default|GetPivotPorte) (CallFunction|LerpDoor _newtrack_0) false false))
              (:Finished
                (if (Variables|Default|GetisOpen)
                  (Variables|Default|SetisOpen false)
                  (else
                    (Variables|Default|SetisOpen true)))
                (Variables|/Game/Blueprints/Player/BP_PlayerController.BP_PlayerController_C|SetcanInteract? (CallFunction|GetPlayerControlleras) true)))
            (else
              (Utilities|FlowControl|Sequence
                (:then_0
                  (Timeline|Door Play))
                (:then_1
                  (bind _newtrack_0_2 (Timeline|Poignee PlayFromStart)
                    (:Update
                      (Transformation|SetRelativeRotation (Variables|Default|GetPivotPoignee) (CallFunction|LerpPoignee _newtrack_0_2) false false))))
                (:then_2
                  (Audio|PlaySound2D (Variables|Default|GetcurrentSound) 1.0 1.0 0.0 0 0)))))
          (else
            (Audio|PlaySound2D (Variables|Default|GetcurrentSoundDoorLock) 1.0 1.0 0.0 0 0)
            (bind _newtrack_0_3 (Timeline|PoigneeLock PlayFromStart)
              (:Update
                (Transformation|SetRelativeRotation (Variables|Default|GetPivotPoignee) (CallFunction|LerpPoignee _newtrack_0_3) false false))
              (:Finished
                (Variables|/Game/Blueprints/Player/BP_PlayerController.BP_PlayerController_C|SetcanInteract? (CallFunction|GetPlayerControlleras) true)))))
        (else
          (goto _label))))))

(event EventBeginPlay
  (Variables|Default|SetstartRotationDoor (Variables|/Script/Engine.SceneComponent|GetRelativeRotation (Variables|Default|GetPivotPorte)))
  (Variables|Default|SetstartRotationPoignee (Variables|/Script/Engine.SceneComponent|GetRelativeRotation (Variables|Default|GetPivotPoignee)))
  (if (Variables|Default|GetinverseRotation)
    (Variables|Default|SetvalueLerp -9e+01)
    (else
      (Variables|Default|SetvalueLerp 9e+01))))

(fn ConstructionScript
  (|CallParentFunction))

(fn LerpDoor
  (params (Alpha :type Float%20%28single-precision%29))
  (bind _startrotationdoor (Variables|Default|GetstartRotationDoor))
  (bind (_roll _pitch _yaw) (Math|Rotator|BreakRotator _startrotationdoor))
  (return (Math|Rotator|Lerp(Rotator) _startrotationdoor (Math|Rotator|MakeRotator _roll _pitch (- _yaw (Variables|Default|GetvalueLerp))) Alpha)))

(fn LerpPoignee
  (params (Alpha :type Float%20%28single-precision%29))
  (bind _startrotationpoignee (Variables|Default|GetstartRotationPoignee))
  (bind (_roll _pitch _yaw) (Math|Rotator|BreakRotator _startrotationpoignee))
  (return (Math|Rotator|Lerp(Rotator) _startrotationpoignee (Math|Rotator|MakeRotator (- _roll 45.0) _pitch _yaw) Alpha)))

(fn AddEffectInteract)