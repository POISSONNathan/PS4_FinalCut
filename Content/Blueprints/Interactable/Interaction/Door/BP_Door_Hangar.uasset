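; Hangar door interactable that sends the player to the Entrepot level behind a loading screen.
; Its interact effect creates a loading screen widget, adds it to the viewport and stores it, then triggers the teleport event.
; That event waits briefly, removes the widget and opens the level by name.
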(event Custom|TpHangar
  (Utilities|FlowControl|Delay 2.0)
  (Widget|RemovefromParent (Variables|Default|GetcurrentUi))
  (Game|OpenLevel(byName) "Entrepot"))

(fn ConstructionScript
  (|CallParentFunction))

(fn AddEffectInteract
  (bind _returnvalue (UserInterface|CreateWidget "/Game/Blueprints/Player/WBP_LoadingScreen.WBP_LoadingScreen_C"))
  (UserInterface|Viewport|AddtoViewport _returnvalue 0)
  (Variables|Default|SetcurrentUi _returnvalue)
  (CallFunction|TpHangar))