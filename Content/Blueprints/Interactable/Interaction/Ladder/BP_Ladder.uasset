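; BP_Ladder is an interactable ladder that moves the player character upward along world Z.
; Interacting while grounded sets one-way open and on-ladder flags, stops movement, and uses a timeline to lerp the player to TargetPoint.
; When the timeline finishes, it binds an event to the player controller's move-forward input and disables gravity.
; GoUp applies only non-negative input, scaled by LadderSpeed; no descent or exit logic appears here.
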(event EventInteractwithObj
  (params (Controller :type BP%20Player%20Controller%20Object%20Reference) (Character :type First%20Person%20Character%20Object%20Reference))
  (if (AI|Components|NavMovement|IsMovingonGround (Variables|/Script/Engine.Character|GetCharacterMovement Character))
    (if (not (Variables|Default|GetisOpen))
      (Variables|Default|SetisOpen true)
      (Variables|/Game/Blueprints/Player/FirstPersonCharacter.FirstPersonCharacter_C|SetonLadder Character true)
      (Components|Movement|StopMovementImmediately (Variables|/Script/Engine.Character|GetCharacterMovement Character))
      (bind _newtrack_0 (Timeline|LerpChar PlayFromStart)
        (:Update
          (Transformation|SetActorLocation (CallFunction|GetPlayerCharacteras) (Math|Vector|Lerp(Vector) (Transformation|GetActorLocation (CallFunction|GetPlayerCharacteras)) (Transformation|GetActorLocation (Variables|Default|GettargetPoint)) _newtrack_0) false false))
        (:Finished
          (Default|BindEventtoMoveForward (CallFunction|GetPlayerControlleras) true (EventDispatchers|CreateEvent :!event GoUp))
          (Default|SetGravity (CallFunction|GetPlayerCharacteras) false))))))

(fn ConstructionScript)

(fn GoUp
  (params (Axis :type Float%20%28single-precision%29))
  (if (>= Axis 0.0)
    (Transformation|AddActorWorldOffset (CallFunction|GetPlayerCharacteras) (Math|Vector|MakeVector 0.0 0.0 (* Axis (Variables|Default|GetLadderSpeed))))))