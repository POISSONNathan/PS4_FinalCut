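; BP_PossessObject is an interactable that moves the player's view onto itself for observing or possessing the object.
; InteractwithObj blends the camera to it, unbinds look-up events, shows the observable-object UI with its name and tutorial images, and takes input.
; The interaction button calls LeaveObject, which blends back to the character, removes the UI and restores bindings and interaction.
; Empty AddEffectInteract and AddEffectLeaveObject functions serve as effect hooks.
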(event Custom|LeaveObject
  (if (Variables|Default|GetisOpen)
    (Game|Player|SetViewTargetwithBlend (CallFunction|GetPlayerControlleras) (CallFunction|GetPlayerCharacteras) 1.0 "VTBlend_Linear" 0.0 false)
    (Input|DisableInput (CallFunction|GetPlayerControlleras))
    (Widget|RemovefromParent (Variables|/Game/Blueprints/Player/BP_PlayerController.BP_PlayerController_C|GetuiObservableObject (CallFunction|GetPlayerControlleras)))
    (Utilities|FlowControl|Delay 1.0)
    (Variables|Default|SetisOpen false)
    (Variables|/Game/Blueprints/Player/BP_PlayerController.BP_PlayerController_C|SetcanInteract? (CallFunction|GetPlayerControlleras) true)
    (Default|ResetBinding (CallFunction|GetPlayerControlleras))
    (CallFunction|AddEffectLeaveObject)))

(event EventInteractwithObj
  (params (Controller :type BP%20Player%20Controller%20Object%20Reference) (Character :type First%20Person%20Character%20Object%20Reference))
  (bind _asbp_player_controller (CallFunction|GetPlayerControlleras))
  (bind _uiobservableobject (Variables|/Game/Blueprints/Player/BP_PlayerController.BP_PlayerController_C|GetuiObservableObject _asbp_player_controller))
  (if (not (Variables|Default|GetisOpen))
    (Game|Player|SetViewTargetwithBlend Controller self 1.0 "VTBlend_Linear" 0.0 false)
    (Variables|Default|SetisOpen true)
    (Utilities|FlowControl|Delay 1.0)
    (EventDispatchers|UnbindallEventsfromLookUp (CallFunction|GetPlayerControlleras))
    (UserInterface|Viewport|AddtoViewport _uiobservableobject 0)
    (Default|ChangeImageNameObject _uiobservableobject (Variables|Default|GetimageNameObject))
    (Default|ChangeTutoObject _uiobservableobject (Variables|Default|GetimageTutoObject))
    (Input|EnableInput (CallFunction|GetPlayerControlleras))
    (CallFunction|AddEffectInteract)))

(event EventBeginPlay)

(event Input|ActionEvents|InputActionInteractionButton
  (params (Key :type Key%20Structure :default "None"))
  (:Pressed
    (CallFunction|LeaveObject)))

(fn ConstructionScript
  (|CallParentFunction))

(fn AddEffectInteract)

(fn AddEffectLeaveObject)