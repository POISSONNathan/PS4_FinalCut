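; Digicode keypad, an interactable possess object where the player enters a code to match FinalCode.
; ChangeCode appends input up to four characters and shows it on a text render.
; ValideCode sets GoodCode and leaves the object on a match, otherwise it clears the entry through ResetCode.
; Interact and leave effect functions toggle the mouse cursor and click events on the player controller.
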(event Custom|ChangeCode
  (params (B :type String))
  (if (< (Utilities|String|Len (Variables|Default|GetcurrentCode)) 4)
    (Variables|Default|SetcurrentCode (Utilities|String|Append (Variables|Default|GetcurrentCode) B))
    (Rendering|Components|TextRender|SetText (Variables|Default|GetTextRender) (Utilities|Text|ToText(String) (Variables|Default|GetcurrentCode)))))

(event Custom|ResetCode
  (Variables|Default|SetcurrentCode "")
  (Rendering|Components|TextRender|SetText (Variables|Default|GetTextRender) (Utilities|Text|ToText(String) (Variables|Default|GetcurrentCode))))

(event Custom|ValideCode
  (if (Utilities|Enum|Equal(Enum) (Variables|Default|GetcurrentCode) (Variables|Default|GetfinalCode))
    (Variables|Default|SetgoodCode true)
    (CallFunction|LeaveObject)
    (else
      (CallFunction|ResetCode))))

(event EventBeginPlay
  (Rendering|Components|TextRender|SetText (Variables|Default|GetTextRender) (Utilities|Text|ToText(String) "")))

(fn ConstructionScript
  (|CallParentFunction))

(fn AddEffectInteract
  (bind _asbp_player_controller (CallFunction|GetPlayerControlleras))
  (Variables|/Script/Engine.PlayerController|SetbShowMouseCursor _asbp_player_controller true)
  (Variables|/Script/Engine.PlayerController|SetbEnableClickEvents _asbp_player_controller true))

(fn AddEffectLeaveObject
  (bind _asbp_player_controller (CallFunction|GetPlayerControlleras))
  (Variables|/Script/Engine.PlayerController|SetbShowMouseCursor _asbp_player_controller false)
  (Variables|/Script/Engine.PlayerController|SetbEnableClickEvents _asbp_player_controller false))