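; BP_CodeButton is a clickable key for a digicode keypad, acting as either a value key, a validate key or a reset key.
; Its construction script writes the key's value onto its text render component.
; On click it plays a sound, then calls the player controller to add its value or, when flagged Valide or Reset, to validate or reset the code through one shared boolean call.
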(event MouseInput|EventActorOnClicked
  (params (ButtonPressed :type Key%20Structure :default "None"))
  (Audio|PlaySound2D (Variables|Default|GetsoundButton) 1.0 1.0 0.0 0 0)
  (if (or (Variables|Default|GetValide) (Variables|Default|GetReset))
    (if (Variables|Default|GetValide)
      (Default|CallResetorValideDigicode (CallFunction|GetPlayerControlleras) true)
      (else
        (Default|CallResetorValideDigicode (CallFunction|GetPlayerControlleras) false)))
    (else
      (Default|CallAddKeyDigicode (CallFunction|GetPlayerControlleras) (Variables|Default|GetvalueButtonText)))))

(fn ConstructionScript
  (Rendering|Components|TextRender|SetText (Variables|Default|GetTextRender) (Utilities|Text|ToText(String) (Variables|Default|GetvalueButtonText))))