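; BP_CodeButton is a clickable key for a digicode, serving as a value, validate or reset button.
; On click, its Valide and Reset flags choose which CodeMaster function runs: ValideCode, ResetCode, or ChangeCode with the button's value.
; Validation is skipped once CodeMaster's GoodCode is set.
; The construction script writes the button's value onto its TextRender label.
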(event MouseInput|EventActorOnClicked
  (params (ButtonPressed :type Key%20Structure :default "None"))
  (if (or (Variables|Default|GetValide) (Variables|Default|GetReset))
    (if (Variables|Default|GetValide)
      (if (not (Variables|/Game/Blueprints/Interaction/PossessObject/Digicode/BP_Digicode.BP_Digicode_C|GetgoodCode (Variables|Default|GetcodeMaster)))
        (Default|ValideCode (Variables|Default|GetcodeMaster)))
      (else
        (Default|ResetCode (Variables|Default|GetcodeMaster))))
    (else
      (Default|ChangeCode (Variables|Default|GetcodeMaster) (Variables|Default|GetvalueButtonText)))))

(fn ConstructionScript
  (Rendering|Components|TextRender|SetText (Variables|Default|GetTextRender) (Utilities|Text|ToText(String) (Variables|Default|GetvalueButtonText))))