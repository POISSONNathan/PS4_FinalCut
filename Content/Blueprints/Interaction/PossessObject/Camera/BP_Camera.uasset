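; BP_Camera is an interactable camera, apparently possessable, that the player can pan horizontally.
; Its interact effect rebinds the player controller's turn event, and turn input sets left or right flags while the left mouse button is held.
; Tick steps the CameraToSee yaw by a fixed, frame-rate-dependent amount, clamped to an arc around its starting rotation.
; Releasing the button clears both flags.
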(event Custom|TurnFunction
  (params (Val :type Float%20%28single-precision%29))
  ;[1 1 1] Turn camera
  (if (Variables|Default|GetleftMouseClick)
    (Variables|Default|SetisRotateRight (> Val 0.0))
    (Variables|Default|SetisRotateLeft (< Val 0.0))))

(event Custom|ResetRotate
  ;[1 1 1] Turn camera
  (Variables|Default|SetisRotateRight false)
  (Variables|Default|SetisRotateLeft false))

(event EventTick
  (params (DeltaSeconds :type Float%20%28single-precision%29))
  (bind _cameratosee (Variables|Default|GetCameraToSee))
  (bind _startrotationcamera (Variables|Default|GetstartRotationCamera))
  (bind _startrotationcamera_2 (Variables|Default|GetstartRotationCamera))
  (bind _cameratosee_2 (Variables|Default|GetCameraToSee))
  (bind _yaw (Math|Rotator|BreakRotator _startrotationcamera))
  (bind _yaw_2 (Math|Rotator|BreakRotator _startrotationcamera_2))
  (bind _relativerotation (Variables|/Script/Engine.SceneComponent|GetRelativeRotation _cameratosee))
  (bind _relativerotation_2 (Variables|/Script/Engine.SceneComponent|GetRelativeRotation _cameratosee_2))
  (bind (_roll _pitch _yaw_3) (Math|Rotator|BreakRotator _relativerotation_2))
  (bind (_roll_2 _pitch_2 _yaw_4) (Math|Rotator|BreakRotator _relativerotation))
  ;[1 1 1] Turn camera
  (Utilities|FlowControl|Sequence
    (:then_0
      (if (Variables|Default|GetisRotateLeft)
        (Transformation|SetRelativeRotation (Variables|Default|GetCameraToSee) (Math|Rotator|MakeRotator _roll _pitch (Math|Float|ClampAngle (+ _yaw_3 -2.0) (- _yaw 45.0) (+ _yaw 45.0))) false false)))
    (:then_1
      (if (Variables|Default|GetisRotateRight)
        (Transformation|SetRelativeRotation (Variables|Default|GetCameraToSee) (Math|Rotator|MakeRotator _roll_2 _pitch_2 (Math|Float|ClampAngle (+ _yaw_4 2.0) (- _yaw_2 45.0) (+ _yaw_2 45.0))) false false)))))

(event EventBeginPlay
  (|CallParentFunction)
  (Variables|Default|SetstartRotationCamera (Variables|/Script/Engine.SceneComponent|GetRelativeRotation (Variables|Default|GetCameraToSee))))

(event Input|MouseEvents|LeftMouseButton
  (params (Key :type Key%20Structure :default "None"))
  ;[1 1 1] Turn camera
  (:Pressed
    (Variables|Default|SetleftMouseClick true))
  (:Released
    (Variables|Default|SetleftMouseClick false)
    (CallFunction|ResetRotate)))

(fn ConstructionScript
  (|CallParentFunction))

(fn AddEffectInteract
  (Default|BindEventtoTurn (CallFunction|GetPlayerControlleras) true (EventDispatchers|CreateEvent :!event Custom|TurnFunction)))