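; BP_Closet is an interactable closet whose two doors swing open when the player interacts with it.
; InteractwithObj stores both doors' starting rotations, destroys the Sphere component and clears SphereCanAppear.
; The LerpDoor timeline then interpolates each door's relative yaw a quarter turn in opposite directions.
; The event has no closing branch, and the construction script only calls its parent.
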(event EventInteractwithObj
  (params (Controller :type BP%20Player%20Controller%20Object%20Reference) (Character :type First%20Person%20Character%20Object%20Reference))
  (Variables|Default|SetleftDoorStartRotation (Variables|/Script/Engine.SceneComponent|GetRelativeRotation (Variables|Default|GetLeftDoor)))
  (Variables|Default|SetrightDoorStartRotation (Variables|/Script/Engine.SceneComponent|GetRelativeRotation (Variables|Default|GetRightDoor)))
  (Components|DestroyComponent (Variables|Default|GetSphere))
  (Variables|Default|SetsphereCanAppear false)
  (bind _newtrack_0 (Timeline|LerpDoor Play)
    (:Update
      (Transformation|SetRelativeRotation (Variables|Default|GetLeftDoor) (Math|Rotator|Lerp(Rotator) (Variables|Default|GetleftDoorStartRotation) (Math|Rotator|MakeRotator (.Roll (Math|Rotator|BreakRotator (Variables|Default|GetleftDoorStartRotation))) (.Pitch (Math|Rotator|BreakRotator (Variables|Default|GetleftDoorStartRotation))) (+ (.Yaw (Math|Rotator|BreakRotator (Variables|Default|GetleftDoorStartRotation))) 9e+01)) _newtrack_0) false false)
      (Transformation|SetRelativeRotation (Variables|Default|GetRightDoor) (Math|Rotator|Lerp(Rotator) (Variables|Default|GetrightDoorStartRotation) (Math|Rotator|MakeRotator (.Roll (Math|Rotator|BreakRotator (Variables|Default|GetrightDoorStartRotation))) (.Pitch (Math|Rotator|BreakRotator (Variables|Default|GetrightDoorStartRotation))) (+ (.Yaw (Math|Rotator|BreakRotator (Variables|Default|GetrightDoorStartRotation))) -9e+01)) _newtrack_0) false false))))

(fn ConstructionScript
  (|CallParentFunction))