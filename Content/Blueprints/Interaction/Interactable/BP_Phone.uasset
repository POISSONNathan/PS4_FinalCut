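; BP_Phone is an interactable phone that holds the player in place while its sound plays.
; On interaction it disables the character's movement, hides its R component and plays PhoneSound as a 2D sound.
; After a fixed five-second delay, not tied to the sound's length, it re-enables CanInteract on the player controller, restores walking and shows R again.
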(event EventInteractwithObj
  (params (Controller :type BP%20Player%20Controller%20Object%20Reference) (Character :type First%20Person%20Character%20Object%20Reference))
  (bind _charactermovement (Variables|/Script/Engine.Character|GetCharacterMovement Character))
  (Pawn|Components|CharacterMovement|SetMovementMode _charactermovement "MOVE_None" 0)
  (Rendering|SetVisibility (Variables|Default|Getr) false false)
  (Audio|PlaySound2D "/Game/MP3/PhoneCall/PhoneSound.PhoneSound" 1.0 1.0 0.0 0 0)
  (Utilities|FlowControl|Delay 5.0)
  (Variables|/Game/Blueprints/Player/BP_PlayerController.BP_PlayerController_C|SetcanInteract? (CallFunction|GetPlayerControlleras) true)
  (Pawn|Components|CharacterMovement|SetMovementMode _charactermovement "MOVE_Walking" 0)
  (Rendering|SetVisibility (Variables|Default|Getr) true false))

(fn ConstructionScript
  (|CallParentFunction))