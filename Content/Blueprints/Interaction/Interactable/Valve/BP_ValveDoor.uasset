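; BP_ValveDoor is a code check for a valve door that currently only prints a debug message on success.
; ChangeCode appends each incoming item to CurrentCode and compares it with the DoorCode entry at that position.
; A full match prints the message and clears the input.
; A mismatch clears it only when the item equals the code's first entry, without keeping that item as a new start.
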(event Custom|ChangeCode
  (params (NewItem :type Integer%20%28by%20ref%29))
  (Utilities|Array|Add (Variables|Default|GetcurrentCode) NewItem)
  (if (== (Utilities|Array|Get(acopy) (Variables|Default|GetdoorCode) (- (Utilities|Array|Length (Variables|Default|GetcurrentCode)) 1)) NewItem)
    (if (Utilities|Array|Identical (Variables|Default|GetdoorCode) (Variables|Default|GetcurrentCode))
      (Development|PrintString "GOOD CODE")
      (Utilities|Array|Clear (Variables|Default|GetcurrentCode)))
    (elif (== NewItem (Utilities|Array|Get(acopy) (Variables|Default|GetdoorCode)))
      (Utilities|Array|Clear (Variables|Default|GetcurrentCode)))))

(fn ConstructionScript)