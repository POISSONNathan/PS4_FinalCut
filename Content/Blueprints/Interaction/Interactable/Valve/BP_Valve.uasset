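; BP_Valve is an interactable valve that turns and reports its value to a linked door.
; On interaction, a timeline rolls the pivot 90 degrees from its current rotation.
; When the turn finishes, it re-enables the interacting controller's CanInteract flag and passes the valve's value to the door's ChangeCode.
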(event EventInteractwithObj
  (params (Controller :type BP%20Player%20Controller%20Object%20Reference) (Character :type First%20Person%20Character%20Object%20Reference))
  (Variables|Default|SetstartRotation (Variables|/Script/Engine.SceneComponent|GetRelativeRotation (Variables|Default|GetPivot)))
  (bind _newtrack_0 (Timeline|Rotate PlayFromStart)
    (:Update
      (Transformation|SetRelativeRotation (Variables|Default|GetPivot) (Math|Rotator|Lerp(Rotator) (Variables|Default|GetstartRotation) (Math|Rotator|MakeRotator (+ (.Roll (Math|Rotator|BreakRotator (Variables|Default|GetstartRotation))) 9e+01) (.Pitch (Math|Rotator|BreakRotator (Variables|Default|GetstartRotation))) (.Yaw (Math|Rotator|BreakRotator (Variables|Default|GetstartRotation)))) _newtrack_0) false false))
    (:Finished
      (Variables|/Game/Blueprints/Player/BP_PlayerController.BP_PlayerController_C|SetcanInteract? Controller true)
      (Default|ChangeCode (Variables|Default|Getdoor) (Variables|Default|GetvalueValve)))))

(fn ConstructionScript
  (|CallParentFunction))