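; BP_Drawers is an interactable drawer that slides open or closed when the player interacts with it.
; On BeginPlay it stores the actor's start location and the EndPosition component's world location, then hides that component, which uses a translucent material.
; Interaction plays or reverses the OpenDrawer timeline, lerping the actor between both points.
; On finish it flips IsOpen and re-enables CanInteract on the player controller.
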(event EventInteractwithObj
  (params (Controller :type BP%20Player%20Controller%20Object%20Reference) (Character :type First%20Person%20Character%20Object%20Reference))
  (if (Variables|Default|GetisOpen)
    (bind _newtrack_0 (Timeline|OpenDrawer ReverseFromEnd)
      (:Update
        (Transformation|SetActorLocation (Math|Vector|Lerp(Vector) (Variables|Default|GetstartPos) (Variables|Default|GetendPos) _newtrack_0) false false))
      (:Finished
        (if (Variables|Default|GetisOpen)
          (Variables|Default|SetisOpen false)
          (else
            (Variables|Default|SetisOpen true)))
        (Variables|/Game/Blueprints/Player/BP_PlayerController.BP_PlayerController_C|SetcanInteract? (CallFunction|GetPlayerControlleras) true)))
    (else
      (Timeline|OpenDrawer PlayFromStart))))

(event EventBeginPlay
  (Variables|Default|SetstartPos (Transformation|GetActorLocation))
  (Variables|Default|SetendPos (Transformation|GetWorldLocation (Variables|Default|GetendPosition)))
  (Rendering|SetVisibility (Variables|Default|GetendPosition) false false))

(fn ConstructionScript
  (Rendering|Material|SetMaterial (Variables|Default|GetendPosition) 0 "/Game/Blueprints/Interaction/Interactable/M_TransclucentObject.M_TransclucentObject"))