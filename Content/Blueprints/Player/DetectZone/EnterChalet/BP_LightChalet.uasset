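; BP_LightChalet is a chalet light actor that acts as either a point light or a spot light and removes itself when the cottage is entered.
; The construction script shows only the selected light type.
; BeginPlay destroys the unused light component and binds to the player controller's enter-cottage event.
; When that event fires, the remaining light component is destroyed, leaving the actor without either light.
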(event Custom|EventEnterCottage
  (if (Variables|Default|GetpointLight?)
    (Components|DestroyComponent (Variables|Default|GetPointLight))
    (else
      (Components|DestroyComponent (Variables|Default|GetSpotLight)))))

(event EventBeginPlay
  (EventDispatchers|BindEventtoEnterCottage (CallFunction|GetPlayerControlleras) (EventDispatchers|CreateEvent :!event Custom|EventEnterCottage))
  (if (Variables|Default|GetpointLight?)
    (Components|DestroyComponent (Variables|Default|GetSpotLight))
    (else
      (Components|DestroyComponent (Variables|Default|GetPointLight)))))

(fn ConstructionScript
  (if (Variables|Default|GetpointLight?)
    (Rendering|SetVisibility (Variables|Default|GetSpotLight) false false)
    (Rendering|SetVisibility (Variables|Default|GetPointLight) true false)
    (else
      (Rendering|SetVisibility (Variables|Default|GetSpotLight) true false)
      (Rendering|SetVisibility (Variables|Default|GetPointLight) false false))))