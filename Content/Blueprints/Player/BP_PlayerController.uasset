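; Player controller that drives first-person interaction, look input and a simple key inventory, and creates the player UI on BeginPlay.
; Each tick a short camera line trace caches the targeted BP_MasterInteractable, which the InteractionButton triggers when interaction is allowed.
; Turn and LookUp axes fire dispatchers whose handlers can be swapped, with ResetBinding restoring the defaults.
; ClearInventory resets the inventory flags and hides the character's key.
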(event EventBeginPlay
  (CallFunction|ResetBinding)
  (bind _returnvalue (UserInterface|CreateWidget "/Game/Blueprints/Player/WBP_PlayerUI.WBP_PlayerUI_C"))
  (bind _output_get (Variables|Default|SetmyUI _returnvalue))
  (UserInterface|Viewport|AddtoViewport _output_get 0))

(event EventTick
  (params (DeltaSeconds :type Float%20%28single-precision%29))
  (bind _out_hit_hit_actor (CallFunction|CreateLineTrace))
  (bind _asbp_master_interactable (Utilities|Casting|CastToBP_MasterInteractable _out_hit_hit_actor)
    (:then
      (Variables|Default|SetcurrentObjectInteract _asbp_master_interactable))
    (:CastFailed
      (Variables|Default|SetcurrentObjectInteract 0))))

(event Input|ActionEvents|InputActionInteractionButton
  (params (Key :type Key%20Structure))
  (:Pressed
    (Variables|Default|GetcurrentObjectInteract
      (:then
        (if (Variables|Default|GetcanInteract?)
          (Default|InteractwithObj (Variables|Default|GetcurrentObjectInteract) self (CallFunction|GetPlayerCharacteras))))
      (:else))))

(event Input|AxisEvents|InputAxisTurn
  (params (AxisValue :type Float%20%28single-precision%29))
  (Default|CallTurn AxisValue))

(event Input|AxisEvents|InputAxisLookUp
  (params (AxisValue :type Float%20%28single-precision%29))
  (Default|CallLookUp AxisValue))

(fn ConstructionScript)

(fn CreateLineTrace
  (bind _asfirst_person_character (CallFunction|GetPlayerCharacteras))
  (bind _firstpersoncamera (Variables|/Game/Blueprints/Player/FirstPersonCharacter.FirstPersonCharacter_C|GetFirstPersonCamera _asfirst_person_character))
  (bind _returnvalue (Transformation|GetWorldLocation _firstpersoncamera))
  (bind _outhit (Collision|LineTraceByChannel _returnvalue (+ _returnvalue (* (Math|Vector|GetForwardVector _firstpersoncamera) 2e+02)) "TraceTypeQuery1" false 0 "None"))
  (return (.hitactor _outhit)))

(fn BindEventtoTurn
  (params (Clear :type Boolean) (Event :type Delegate%20%28by%20ref%29))
  (Utilities|FlowControl|Sequence
    (:then_0
      (if Clear
        (EventDispatchers|UnbindallEventsfromTurn)))
    (:then_1
      (EventDispatchers|BindEventtoTurn Event))))

(fn BindEventtoLookUp
  (params (Clear :type Boolean) (Event1 :type Delegate%20%28by%20ref%29))
  (Utilities|FlowControl|Sequence
    (:then_0
      (if Clear
        (EventDispatchers|UnbindallEventsfromLookUp)))
    (:then_1
      (EventDispatchers|BindEventtoLookUp Event1))))

(fn ResetBinding
  (CallFunction|BindEventtoTurn true (EventDispatchers|CreateEvent (CallFunction|GetPlayerCharacteras) :!event PlayerTurn))
  (CallFunction|BindEventtoLookUp true (EventDispatchers|CreateEvent (CallFunction|GetPlayerCharacteras) :!event PlayerLookUp)))

(fn ClearInventory
  (Utilities|FlowControl|Sequence
    (:then_0
      (Variables|Default|SetfullInventory false))
    (:then_1
      (Variables|Default|SetgetKey? false)
      (Rendering|SetVisibility (Variables|/Game/Blueprints/Player/FirstPersonCharacter.FirstPersonCharacter_C|Getkey (CallFunction|GetPlayerCharacteras)) false false))))