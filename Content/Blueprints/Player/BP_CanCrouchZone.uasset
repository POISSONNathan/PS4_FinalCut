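; BP_CanCrouchZone is a trigger volume that lets the first-person character crouch only while inside it.
; Entering the box shows a "Press CTRL to crouch" prompt on the player's UI and enables input on the actor, so Left Ctrl calls Crouch on the player.
; Leaving clears the prompt, disables that input and forces UnCrouch, with no handling for key release.
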(event OnComponentBeginOverlap(Box_0)
  (params (OverlappedComponent :type Primitive%20Component%20Object%20Reference) (OtherActor :type Actor%20Object%20Reference) (OtherComp :type Primitive%20Component%20Object%20Reference) (OtherBodyIndex :type Integer) (bFromSweep :type Boolean) (SweepResult :type Hit%20Result%20Structure%20%28by%20ref%29))
  (Utilities|Casting|CastToFirstPersonCharacter OtherActor)
  (Default|SetInformationText (Variables|/Game/Blueprints/Player/BP_PlayerController.BP_PlayerController_C|GetmyUI (CallFunction|GetPlayerControlleras)) "Press CTRL to crouch")
  (Variables|Default|SetisOverlap true)
  (Input|EnableInput (CallFunction|GetPlayerControlleras)))

(event OnComponentEndOverlap(Box_0)
  (params (OverlappedComponent :type Primitive%20Component%20Object%20Reference) (OtherActor :type Actor%20Object%20Reference) (OtherComp :type Primitive%20Component%20Object%20Reference) (OtherBodyIndex :type Integer))
  (Utilities|Casting|CastToFirstPersonCharacter OtherActor)
  (Default|SetInformationText (Variables|/Game/Blueprints/Player/BP_PlayerController.BP_PlayerController_C|GetmyUI (CallFunction|GetPlayerControlleras)))
  (Variables|Default|SetisOverlap false)
  (Input|DisableInput (CallFunction|GetPlayerControlleras))
  (Character|UnCrouch (CallFunction|GetPlayerCharacteras)))

(event Input|KeyboardEvents|LeftCtrl
  (params (Key :type Key%20Structure :default "None"))
  (:Pressed
    (if (Variables|Default|GetisOverlap)
      (Character|Crouch (CallFunction|GetPlayerCharacteras)))))

(fn ConstructionScript
  (|CallParentFunction))